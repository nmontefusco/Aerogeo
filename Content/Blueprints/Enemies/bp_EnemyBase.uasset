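; Base enemy actor that sweeps in on spawn, patrols back and forth, and damages the player on contact.
; BeginPlay registers it in bp_Gamemode's LiveEnemies, randomizes speed and direction, and runs a timeline slide along -Y before enabling Tick movement on Z.
; Hits against non-enemies reverse direction.
; Damage sets Health to clamped Damage minus Health (operands reversed); at zero it decrements the count and destroys itself.
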(event EventTick
  (params (DeltaSeconds :type Float%20%28single-precision%29))
  ;[1 1 1] Movement
  (if (Variables|Default|GetIs_MoveEnabled)
    (Transformation|SetActorLocation (+ (Transformation|GetActorLocation) (* (Math|Vector|RotateVector (Math|Vector|MakeVector 0.0 0.0 (* (Variables|Floats|GetMove_Speed) (Math|Float|SelectFloat 1.0 -1.0 (Variables|Default|GetIs_MoveDirection)))) "0, 0, 0") DeltaSeconds)) true false)))

(event EventBeginPlay
  ;[1 1 1] Control For Random Move Direction
  (bind _asbp_gamemode (Utilities|Casting|CastTobp_Gamemode (Game|GetGameMode)))
  (bind _output_get (Variables|Default|Setbp_GameMode _asbp_gamemode))
  (Variables|/Game/Blueprints/bp_Gamemode.bp_Gamemode_C|SetLive_Enemies _output_get (+ (Variables|/Game/Blueprints/bp_Gamemode.bp_Gamemode_C|GetLive_Enemies _output_get) 1))
  (Variables|Default|SetIs_MoveDirection (Math|Random|RandomBool))
  (Variables|Floats|SetMove_Speed (Math|Random|RandomFloatinRange 5e+02 1e+03))
  (Variables|Floats|SetSweep_In (Math|Random|RandomFloatinRange 1.2e+03 1.7e+03))
  ;[1 1 1] Spawn Animation
  (Variables|Default|SetSpawn_Location (Transformation|GetActorLocation))
  (bind _speed (Timeline|Spawn_Animation Play)
    (:Update
      (Transformation|SetActorLocation (Math|Vector|Lerp(Vector) (Variables|Default|GetSpawn_Location) (- (Variables|Default|GetSpawn_Location) (Math|Vector|MakeVector 0.0 (Variables|Floats|GetSweep_In) 0.0)) _speed) false false))
    (:Finished
      (Variables|Default|SetIs_MoveEnabled true))))

(event Collision|EventHit
  (params (MyComp :type Primitive%20Component%20Object%20Reference) (Other :type Actor%20Object%20Reference) (OtherComp :type Primitive%20Component%20Object%20Reference) (bSelfMoved :type Boolean) (HitLocation :type Vector :default "0, 0, 0") (HitNormal :type Vector :default "0, 0, 0") (NormalImpulse :type Vector :default "0, 0, 0") (Hit :type Hit%20Result%20Structure%20%28by%20ref%29))
  ;[1 1 1] Death
  (Utilities|Casting|CastTobp_EnemyBase Other
    (:then
      _)
    (:CastFailed
      (Variables|Default|SetIs_MoveDirection (not (Variables|Default|GetIs_MoveDirection)))))
  (bind _asbp_player (Utilities|Casting|CastTobp_Player Other))
  (Game|Damage|ApplyDamage _asbp_player 4e+01 0 0))

(event Game|Damage|EventAnyDamage
  (params (Damage :type Float%20%28single-precision%29) (DamageType :type Damage%20Type%20Object%20Reference) (InstigatedBy :type Controller%20Object%20Reference) (DamageCauser :type Actor%20Object%20Reference))
  (bind _bp_gamemode (Variables|Default|Getbp_GameMode))
  ;[1 1 1] Death
  (Variables|Floats|SetHealth (Math|Float|Clamp(Float) (- Damage (Variables|Floats|GetHealth)) 0.0 (Variables|Floats|GetMax_Health)))
  (if (<= (Variables|Floats|GetHealth) 0.0)
    (Variables|/Game/Blueprints/bp_Gamemode.bp_Gamemode_C|SetLive_Enemies _bp_gamemode (- (Variables|/Game/Blueprints/bp_Gamemode.bp_Gamemode_C|GetLive_Enemies _bp_gamemode) 1))
    (Actor|DestroyActor)))

(fn ConstructionScript
  (Variables|Floats|SetHealth (Variables|Floats|GetMax_Health)))