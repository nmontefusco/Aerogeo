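; Boss enemy Blueprint that repeatedly fires pairs of enemy projectiles.
; Tick calls the parent, then runs a Delay of FireRate, which acts as a repeating timer because calls during the countdown are ignored.
; Each completed delay spawns projectiles at the Top and Bottom components with fixed damage and a velocity along negative Y.
; BeginPlay and the construction script only call the parent.
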(event EventBeginPlay
  (|CallParentFunction))

(event EventTick
  (params (DeltaSeconds :type Float%20%28single-precision%29))
  (|CallParentFunction DeltaSeconds)
  (Utilities|FlowControl|Delay (Variables|Default|GetFire_Rate))
  (Game|SpawnActorfromClass "/Game/Blueprints/Projectiles/bp_ProjectileEnemy.bp_ProjectileEnemy_C" (Transformation|GetWorldTransform (Variables|Default|GetTop)) "Undefined" 0 1e+01 "0.000000,-2000.000000,0.000000" "1.000000,1.000000,1.000000")
  (Game|SpawnActorfromClass "/Game/Blueprints/Projectiles/bp_ProjectileEnemy.bp_ProjectileEnemy_C" (Transformation|GetWorldTransform (Variables|Default|GetBottom)) "Undefined" 0 1e+01 "0.000000,-2000.000000,0.000000" "1.000000,1.000000,1.000000"))

(fn ConstructionScript
  (|CallParentFunction))