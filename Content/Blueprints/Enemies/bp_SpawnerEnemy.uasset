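; Enemy spawner that runs three sequential waves of random enemies, starting each once the game mode reports no live enemies.
; A looping timer runs WaveCheck, which selects the enemy list by WaveIndex and calls BeginWave, then SpawnWave.
; BeginWave writes wave counters to bp_Gamemode, receiving the real count only for the first wave and zero afterward.
; SpawnWave spawns the whole wave at once at fixed X/Y and random Z, then re-arms IsWaveReady.
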(event Custom|WaveCheck
  (if (and (== (Variables|/Game/Blueprints/bp_Gamemode.bp_Gamemode_C|GetLive_Enemies (Variables|Default|GetbpGameMode)) 0) (Variables|Default|GetIs_WaveReady))
    (switch int (Variables|Waves|GetWave_Index)
      (:0
        (CallFunction|BeginWave (Utilities|Array|Get(acopy) (Variables|Default|GetWave_EnemyCount) (Variables|Waves|GetWave_Index)))
        (CallFunction|SpawnWave (Utilities|Array|Get(acopy) (Variables|Default|GetWave_EnemyCount) (Variables|Waves|GetWave_Index)) (Variables|Enemies|GetWave_Enemies1)))
      (:1
        (CallFunction|BeginWave)
        (CallFunction|SpawnWave (Utilities|Array|Get(acopy) (Variables|Default|GetWave_EnemyCount) (Variables|Waves|GetWave_Index)) (Variables|Enemies|GetWave_Enemies2)))
      (:2
        (CallFunction|BeginWave)
        (CallFunction|SpawnWave (Utilities|Array|Get(acopy) (Variables|Default|GetWave_EnemyCount) (Variables|Waves|GetWave_Index)) (Variables|Enemies|GetWave_Enemies3))))
    (Variables|Waves|SetWave_Index (+ (Variables|Waves|GetWave_Index) 1))))

(event EventBeginPlay
  ;[1 1 1] Event Begin Play-Spawn Wave
  (bind _asbp_gamemode (Utilities|Casting|CastTobp_Gamemode (Game|GetGameMode)))
  (Variables|Default|SetbpGameMode _asbp_gamemode)
  (bind _returnvalue (Utilities|Time|SetTimerbyFunctionName 0 "WaveCheck" 0.5 true))
  (Variables|Default|SetWave_Timer _returnvalue))

(fn ConstructionScript)

(fn BeginWave
  (params (WaveTotal :type Integer))
  (bind _bpgamemode (Variables|Default|GetbpGameMode))
  (Variables|Default|SetIs_WaveReady false)
  (Variables|Waves|SetWave_Active 0)
  (Variables|/Game/Blueprints/bp_Gamemode.bp_Gamemode_C|SetMax_Waves _bpgamemode WaveTotal)
  (Variables|/Game/Blueprints/bp_Gamemode.bp_Gamemode_C|SetActive_Waves _bpgamemode WaveTotal))

(fn SpawnWave
  (params (WaveTotal :type Integer) (WaveEnemies :type Array%20of%20Bp%20Enemy%20Base%20Class%20References))
  (bind _bpgamemode (Variables|Default|GetbpGameMode))
  (bind _enemy_spawnmin (Variables|/Game/Blueprints/bp_Gamemode.bp_Gamemode_C|GetEnemy_SpawnMin _bpgamemode))
  (for _index (range 0 (+ WaveTotal 1))
    (if (> WaveTotal (Variables|Waves|GetWave_Active))
      (if (not (Variables|Default|GetIs_WaveReady))
        (Game|SpawnActorfromClass (Utilities|Array|Get(acopy) WaveEnemies (Math|Random|RandomInteger (Utilities|Array|Length WaveEnemies))) (Math|Transform|MakeTransform (Math|Vector|MakeVector (.x _enemy_spawnmin) (.y _enemy_spawnmin) (Math|Random|RandomFloatinRange (.z _enemy_spawnmin) (.z (Variables|/Game/Blueprints/bp_Gamemode.bp_Gamemode_C|GetEnemy_SpawnMax _bpgamemode))))) "Undefined" 0 0)
        (Variables|Waves|SetWave_Active (+ (Variables|Waves|GetWave_Active) 1)))
      (else
        (Variables|Default|SetIs_WaveReady true)))))