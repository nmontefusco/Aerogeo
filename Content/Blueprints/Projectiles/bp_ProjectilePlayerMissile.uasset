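; Player missile projectile Blueprint with unfinished or disabled homing logic.
; The first bp_Player to overlap its Homing_Box is stored as the target in TempVar while no valid target is held.
; Tick only checks that target's validity.
; The velocity lerp toward the target at IncreasedSpeed is disconnected and has an alpha of zero, so this graph never steers the missile.
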(event OnComponentBeginOverlap(Homing_Box)
  (params (OverlappedComponent :type Primitive%20Component%20Object%20Reference) (OtherActor :type Actor%20Object%20Reference) (OtherComp :type Primitive%20Component%20Object%20Reference) (OtherBodyIndex :type Integer) (bFromSweep :type Boolean) (SweepResult :type Hit%20Result%20Structure%20%28by%20ref%29))
  (bind _asbp_player (Utilities|Casting|CastTobp_Player OtherActor))
  (Utilities|IsValid (Variables|Default|GetTempVar)
    (:Is%20Not%20Valid
      (Variables|Default|SetTempVar _asbp_player))))

(event EventTick
  (params (DeltaSeconds :type Float%20%28single-precision%29))
  (Utilities|IsValid (Variables|Default|GetTempVar)))

(fn ConstructionScript
  (|CallParentFunction))