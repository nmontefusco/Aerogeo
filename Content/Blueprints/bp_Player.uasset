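; Player ship pawn for a shooter, flying in the Y/Z plane after a timeline fly-in on spawn.
; Tick eases input into speeds, moves with sweep, pitches the mesh by vertical speed and counts down fire timers.
; Input-held gates release primary, powerup-spread or missile volleys, though all three spawn calls use the Bp_Player class.
; Any damage is fatal, flagging player death on bp_Gamemode and destroying the actor.
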(event Custom|FireRateControl
  (bind _projectile_spawn (Variables|Default|GetProjectile_Spawn))
  ;[1 1 1] Projectiles
  (Utilities|FlowControl|Sequence
    (:then_0
      (Variables|Floats|SetPrimary_fireRate (- (Variables|Floats|GetPrimary_fireRate) (Variables|Floats|GetDelta_Sec)))
      (if (<= (Variables|Floats|GetPrimary_fireRate) 0.0)
        (Utilities|FlowControl|Gate true
          (:Exit
            (Variables|Floats|SetPrimary_fireRate (Variables|Floats|GetPrimary_fireRatebase))
            (if (not (Variables|Bools|GetIs_Powerup))
              (CallFunction|PrimaryFire _projectile_spawn)
              (else
                (CallFunction|PowerupFire _projectile_spawn (Variables|Default|GetPowershot_Count))))))))
    (:then_1
      (Variables|Floats|SetMissile_fireRate (- (Variables|Floats|GetMissile_fireRate) (Variables|Floats|GetDelta_Sec)))
      (if (<= (Variables|Floats|GetMissile_fireRate) 0.0)
        (Utilities|FlowControl|Gate true
          (:Exit
            (Variables|Floats|SetMissile_fireRate (Variables|Floats|GetMissile_fireRatebase))
            (if (Variables|Bools|GetIs_Missiles)
              (CallFunction|MissileFire (Variables|Default|GetMissile_Count) _projectile_spawn))))))))

(event EventBeginPlay
  ;[1 1 1] Spawn Animation
  (Variables|Floats|SetHealth (Variables|Floats|GetMax_Health))
  (Variables|Floats|SetPitch (.Pitch (Math|Rotator|BreakRotator (Math|Conversions|RotationFromXVector (Variables|/Script/Engine.SceneComponent|GetRelativeLocation (Variables|Default|GetPlayer_Mesh))))))
  (Variables|Default|SetSpawnRotation (Transformation|GetWorldRotation (Variables|Default|GetPlayer_Mesh)))
  (Variables|Default|SetSpawn_Location (Transformation|GetActorLocation))
  (bind _spawn (Timeline|Player_Spawnanim Play)
    (:Update
      (Transformation|SetActorLocation (Math|Vector|Lerp(Vector) (Variables|Default|GetSpawn_Location) (+ (Variables|Default|GetSpawn_Location) "0,1000.000000, 0") _spawn) false false)
      (Transformation|SetRelativeRotation (Variables|Default|GetPlayer_Mesh) (Math|Rotator|Lerp(Rotator) (Variables|Default|GetSpawnRotation) (Math|Rotator|MakeRotator 0.0 (+ (Variables|Floats|GetAnimation_Pitch) (Variables|Floats|GetPitch)) 0.0) _spawn) false false))
    (:Finished
      (Variables|Bools|SetIs_Moving true))))

(event Game|Damage|EventAnyDamage
  (params (Damage :type Float%20%28single-precision%29) (DamageType :type Damage%20Type%20Object%20Reference) (InstigatedBy :type Controller%20Object%20Reference) (DamageCauser :type Actor%20Object%20Reference))
  ;[1 1 1] Player Death
  (Variables|Floats|SetHealth 0.0)
  (if (<= (Variables|Floats|GetHealth) 0.0)
    (bind _asbp_gamemode (Utilities|Casting|CastTobp_Gamemode (Game|GetGameMode)))
    (Variables|/Game/Blueprints/bp_Gamemode.bp_Gamemode_C|SetIs_Playerdead _asbp_gamemode true)
    (Actor|DestroyActor)))

(event EventTick
  (params (DeltaSeconds :type Float%20%28single-precision%29))
  ;[1 1 1] Movement
  (Variables|Floats|SetDelta_Sec DeltaSeconds)
  (if (Variables|Bools|GetIs_Moving)
    (CallFunction|FireRateControl)
    (Utilities|FlowControl|Sequence
      (:then_0
        (bind _returndirection (CallFunction|GetDirection (Variables|Floats|GetVert_Speed) (Input|AxisValues|GetMove_Up)))
        (Variables|Floats|SetVert_Speed _returndirection))
      (:then_1
        (bind _returndirection_2 (CallFunction|GetDirection (Variables|Floats|GetHorz_Speed) (Input|AxisValues|GetMove_Right)))
        (Variables|Floats|SetHorz_Speed _returndirection_2))
      (:then_2
        (Transformation|SetActorLocation (+ (Transformation|GetActorLocation) (Math|Vector|MakeVector 0.0 0.0 (Variables|Floats|GetVert_Speed))) true false)
        (Transformation|SetActorLocation (+ (Transformation|GetActorLocation) (Math|Vector|MakeVector 0.0 (Variables|Floats|GetHorz_Speed) 0.0)) true false)
        (if (> (Variables|Floats|GetHealth) 0.0)
          (Transformation|SetRelativeRotation (Variables|Default|GetPlayer_Mesh) (Math|Interpolation|RInterpTo (Transformation|GetActorRotation) (Math|Rotator|MakeRotator 0.0 (* (Variables|Floats|GetVert_Speed) 4.0) 0.0) (Variables|Floats|GetDelta_Sec) 0.0) false false))))))

(event Input|ActionEvents|InputActionFire
  (params (Key :type Key%20Structure :default "AnyKey"))
  (bind _projectile_spawn (Variables|Default|GetProjectile_Spawn))
  ;[1 1 1] Projectiles
  (:Pressed
    (Utilities|FlowControl|Gate true) ; enters at Open
  )
  (:Released
    (Utilities|FlowControl|Gate true) ; enters at Close
  ))

(event Input|ActionEvents|InputActionMissile
  (params (Key :type Key%20Structure :default "AnyKey"))
  ;[1 1 1] Projectiles
  (:Pressed
    (Utilities|FlowControl|Gate true) ; enters at Open
  )
  (:Released
    (Utilities|FlowControl|Gate true) ; enters at Close
  ))

(fn ConstructionScript)

(fn GetDirection
  (params (Speed :type Float%20%28single-precision%29) (Direction :type Float%20%28single-precision%29))
  (bind _output_get (Variables|Floats|SetCurrent_Speed (Math|Interpolation|FInterpTo Speed (* Direction (Variables|Floats|GetMove_Speed)) (Variables|Floats|GetDelta_Sec) 4.0)))
  (return _output_get))

(fn PrimaryFire
  (params (Spawn_Location :type Scene%20Component%20Object%20Reference))
  (bind _returnvalue (Transformation|GetWorldTransform Spawn_Location))
  (bind (_location _rotation) (Math|Transform|BreakTransform _returnvalue))
  (Game|SpawnActorfromClass "bp_Player_C" (Math|Transform|MakeTransform (Math|Vector|MakeVector (.x _location) (.y _location) (+ (.z _location) (Math|Random|RandomFloatinRange -7e+01 7e+01))) _rotation) "AlwaysSpawn" 0 0))

(fn PowerupFire
  (params (Spawn_Location :type Scene%20Component%20Object%20Reference) (Num_Shots :type Integer))
  (bind _returnvalue (Transformation|GetWorldTransform Spawn_Location))
  (bind _location (Math|Transform|BreakTransform _returnvalue))
  (LocalVariables|SetOffset (/ Num_Shots -2))
  (for _index (range 0 Num_Shots)
    (Game|SpawnActorfromClass "bp_Player_C" (Math|Transform|MakeTransform (Math|Vector|MakeVector (.x _location) (.y _location) (+ (.z _location) (* (Math|Conversions|ToFloat(Integer) (LocalVariables|GetOffset)) 5.0))) (Math|Rotator|MakeRotator (* (Math|Conversions|ToFloat(Integer) (LocalVariables|GetOffset)) 5.0) 0.0 0.0)) "AlwaysSpawn" 0 0)
    (LocalVariables|SetOffset (+ (LocalVariables|GetOffset) 1))))

(fn MissileFire
  (params (Num_Shots :type Integer) (Spawn_Location :type Scene%20Component%20Object%20Reference))
  (bind _returnvalue (Transformation|GetWorldTransform Spawn_Location))
  (bind _location (Math|Transform|BreakTransform _returnvalue))
  (LocalVariables|SetOffset (/ (+ Num_Shots 4) -1))
  (for _index (range 0 Num_Shots)
    (Game|SpawnActorfromClass "bp_Player_C" (Math|Transform|MakeTransform (Math|Vector|MakeVector (.x _location) (.y _location) (+ (.z _location) (* (Math|Conversions|ToFloat(Integer) (LocalVariables|GetOffset)) 5.0))) (Math|Rotator|MakeRotator (* (Math|Conversions|ToFloat(Integer) (LocalVariables|GetOffset)) 5.0) 0.0 0.0)) "AlwaysSpawn" 0 0)
    (LocalVariables|SetOffset (+ (LocalVariables|GetOffset) 4))))